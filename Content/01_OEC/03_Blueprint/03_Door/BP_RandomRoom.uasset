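; BP_RandomRoom is a room that traps the player between two doors until an inside button releases them.
; The player's first overlap with the box trigger closes and locks Door1, then opens Door2 after a short delay, guarded by DoOnce.
; Clicking InsideButton fires the escape event, which opens Door2, waits briefly, then opens and unlocks Door1.
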(event `self.ReceiveBeginPlay`
  ; 탈출 버튼 눌렀을때 문 다 열림
  (add `OecQuestionButton.OnButtonClicked` (`self.Inside_Button`) (delegate `Event_EscapeRoom`)))

(event `Event_EscapeRoom`
  (bind _door_1 (`self.Door_1`))
  ; 탈출 버튼 눌렀을때 문 다 열림
  (`OecDoorBase.SetDoorState` (`self.Door_2`) true)
  (`KismetSystemLibrary.Delay` 1.0)
  (`OecDoorBase.SetDoorState` _door_1 true)
  (`OecDoorBase.SetDoorLocked` _door_1 false))

(event `self.BoxCollision.OnComponentBeginOverlap`
  (params (OverlappedComponent :type "PrimitiveComponent Object Reference") (OtherActor :type "Actor Object Reference") (OtherComp :type "PrimitiveComponent Object Reference") (OtherBodyIndex :type Integer) (bFromSweep :type Boolean) (SweepResult :type "HitResult Structure (by ref)"))
  (bind _door_1 (`self.Door_1`))
  ; 오버랩 됐을때 문1닫히고 문2열림
  (cast `OecPlayerCharacter` OtherActor)
  (`/Engine/EditorBlueprintResources/StandardMacros.DoOnce` false
    (:`Completed`
      (`OecDoorBase.SetDoorState` _door_1 false)
      (`OecDoorBase.SetDoorLocked` _door_1 true)
      (`KismetSystemLibrary.Delay` 1.5)
      (`OecDoorBase.SetDoorState` (`self.Door_2`) true))))

(fn `UserConstructionScript`)